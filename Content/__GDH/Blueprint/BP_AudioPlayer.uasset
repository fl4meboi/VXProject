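; Audio player actor that starts its sound on BeginPlay and visualizes the loudness on its meshes.
; Each playback-percent update reads the sound's cooked amplitude envelope, avoiding Tick.
; The envelope drives the StaticMesh's Z scale and the Emissive parameter of a dynamic MI_EmissiveLight instance on the Sphere.
; When audio finishes, the mesh's Z scale drops to zero, while emissive is not reset.
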(event `self.ReceiveBeginPlay`
  (bind _audio (`self.Audio`))
  (add `AudioComponent.OnAudioPlaybackPercent` _audio (delegate `OnAudioPlayEvent`))
  (add `AudioComponent.OnAudioFinished` _audio (delegate `OnAudioFinish`))
  (add `AudioComponent.OnAudioFinished` (`self.Audio`) (delegate `OnAudioFinish`))
  (bind _returnvalue (`KismetMaterialLibrary.CreateDynamicMaterialInstance` "/Game/__GDH/Metarials/MI_EmissiveLight.MI_EmissiveLight"))
  (bind _output_get (set `self.DM_Emissive` _returnvalue))
  (`PrimitiveComponent.SetMaterial` (`self.Sphere`) 0 _output_get)
  (`AudioComponent.Play` (`self.Audio`) 0.0))

(event `OnAudioPlayEvent`
  (params (PlayingSoundWave :type "SoundWave Object Reference") (PlaybackPercent :type "Float (single-precision)"))
  (bind _outenvelopedata (`AudioComponent.GetCookedEnvelopeData` (`self.Audio`)))
  (`SceneComponent.SetRelativeScale3D` (`self.StaticMesh`) (`KismetMathLibrary.MakeVector` 1.0 1.0 (* _outenvelopedata 10.0)))
  (`MaterialInstanceDynamic.SetScalarParameterValue` (`self.DM_Emissive`) "Emissive" (* _outenvelopedata 4.0)))

(event `OnAudioFinish`
  (`SceneComponent.SetRelativeScale3D` (`self.StaticMesh`) (1.0 1.0 0.0)))

(fn `UserConstructionScript`)