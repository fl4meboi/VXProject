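; Elevator actor whose platform travels between its base and the position of an End component, switching each time the third-person character enters its trigger box.
; A FlipFlop alternates two MoveComponentTo nodes, stopping the opposite move before starting the next.
; The construction script stacks static meshes at intervals of the Floor's height up to End's Z, so the structure scales with the travel height.
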(event `self.TriggerBox.OnComponentBeginOverlap`
  (params (OverlappedComponent :type "PrimitiveComponent Object Reference") (OtherActor :type "Actor Object Reference") (OtherComp :type "PrimitiveComponent Object Reference") (OtherBodyIndex :type Integer) (bFromSweep :type Boolean) (SweepResult :type "HitResult Structure (by ref)"))
  (bind _platform (`self.Platform`))
  (bind _end_location (`KismetMathLibrary.BreakTransform` (`self.End`)))
  (bind _over_time (`self.Over Time`))
  (cast `/Game/ThirdPerson/Blueprints/BP_ThirdPersonCharacter` OtherActor)
  (`/Engine/EditorBlueprintResources/StandardMacros.FlipFlop`
    (:`A`
      (`|ExecutionSequence`
        (:`then_0`
          (goto _label_2 :!via `Stop`))
        (:`then_1`
          (`KismetSystemLibrary.MoveComponentTo` _platform _end_location (struct) false false _over_time :!label _label))))
    (:`B`
      (`|ExecutionSequence`
        (:`then_0`
          (goto _label :!via `Stop`))
        (:`then_1`
          (`KismetSystemLibrary.MoveComponentTo` _platform (0.0 0.0 0.0) (struct) false false _over_time :!label _label_2))))))

(fn `UserConstructionScript`
  (bind _returnvalue (* (.z (`.BoxExtent` (`KismetSystemLibrary.GetComponentBounds` (`self.Floor`)))) 2.0))
  (for _index (range (+ (`KismetMathLibrary.FTrunc` (/ (.z (.location (`self.End`))) _returnvalue)) 1))
    (`AddComponent|NODE_AddStaticMeshComponent-0` :`RelativeTransform` (`KismetMathLibrary.MakeTransform` (`KismetMathLibrary.MakeVector` 0.0 0.0 (* _index _returnvalue))))))